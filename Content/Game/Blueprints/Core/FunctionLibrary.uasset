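; Blueprint function library providing a camera-based interaction trace and a shortcut to the game instance.
; LineTrace casts a Visibility ray forward from player 0's camera, then runs a small zero-length sphere trace at the hit location.
; It returns the sphere trace's result, hit actor and component rather than the line's.
; GetGame returns the game instance cast to the project's Game class.
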(fn LineTrace
  (params (TraceDistance :type Float%20%28single-precision%29) (DrawDebugType :type EDrawDebugTrace%20Enum :default "None"))
  (bind ___worldcontext (LocalVariables|Get__WorldContext))
  (bind _returnvalue (Game|GetPlayerCameraManager ___worldcontext))
  (bind _transformcomponent (Variables|/Script/Engine.PlayerCameraManager|GetTransformComponent _returnvalue))
  (bind _returnvalue_2 (Transformation|GetWorldTransform _transformcomponent))
  (bind (_location _rotation) (Math|Transform|BreakTransform _returnvalue_2))
  (bind _outhit (Collision|LineTraceByChannel (LocalVariables|Get__WorldContext) _location (+ _location (* (Math|Vector|GetForwardVector _rotation) TraceDistance)) "TraceTypeQuery1" false 0 DrawDebugType))
  (bind (_outhit_2 _returnvalue_3) (Collision|SphereTraceByChannel (LocalVariables|Get__WorldContext) (.Location (Collision|BreakHitResult _outhit)) (.Location (Collision|BreakHitResult _outhit)) 8.0 "TraceTypeQuery1" false 0 DrawDebugType))
  (return _returnvalue_3 (.HitActor (Collision|BreakHitResult _outhit_2)) (.HitComponent (Collision|BreakHitResult _outhit_2)) _outhit_2))

(fn GetGame
  (bind _asgame (Utilities|Casting|CastToGame (Game|GetGameInstance (LocalVariables|Get__WorldContext))))
  (return _asgame))