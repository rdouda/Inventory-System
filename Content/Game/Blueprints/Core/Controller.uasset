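; Player controller that creates the player's interface widget and provides keyboard shortcuts for save games.
; On BeginPlay it adds the PlayerInterface widget to the viewport and caches the Game object returned by GetGame.
; The P, L and K keys call that object to save, load and delete the save game, with P also loading immediately after saving.
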(event EventBeginPlay
  (bind _returnvalue (UserInterface|CreateWidget "/Game/Game/Blueprints/UI/PlayerInterface.PlayerInterface_C" self))
  (bind _output_get (Variables|Default|SetPlayerInterface _returnvalue))
  (UserInterface|Viewport|AddtoViewport _output_get 0)
  (bind _game (CallFunction|GetGame))
  (Variables|Default|SetGame _game))

(event Input|KeyboardEvents|P
  (params (Key :type Key%20Structure :default "None"))
  (:Pressed
    (Default|MakeSaveGame (Variables|Default|GetGame))
    (Default|LoadSaveGame (Variables|Default|GetGame))))

(event Input|KeyboardEvents|L
  (params (Key :type Key%20Structure :default "None"))
  (:Pressed
    (Default|LoadSaveGame (Variables|Default|GetGame))))

(event Input|KeyboardEvents|K
  (params (Key :type Key%20Structure :default "None"))
  (:Pressed
    (Default|DeleteSaveGame (Variables|Default|GetGame))))

(fn ConstructionScript)