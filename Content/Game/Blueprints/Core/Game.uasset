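; Core game Blueprint that saves, loads and deletes a single-slot WorldSaveGame and exposes the mouse sensitivity setting.
; Saving gathers data from the player pawn and all ItemBase and Interactable actors through message calls.
; Loading destroys and respawns items from saved class and transform, restores interactables in place by matching ObjectName, then passes saved data to the player pawn.
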(event Custom|MakeSaveGame
  (bind _returnvalue (SaveGame|CreateSaveGameObject "/Game/Game/Blueprints/SaveGame/WorldSaveGame.WorldSaveGame_C"))
  (Variables|Default|SetSaveGame _returnvalue)
  (CallFunction|CollectPlayerData)
  (CallFunction|CollectWorldData)
  (bind _returnvalue_2 (SaveGame|SaveGametoSlot (Variables|Default|GetSaveGame) (Variables|Default|GetSaveGameSlotName)))
  (if _returnvalue_2
    (Development|PrintString "Game Saved." true false "(R=0.116623,G=1.000000,B=0.000000,A=1.000000)")))

(event Custom|LoadSaveGame
  (bind _returnvalue (SaveGame|DoesSaveGameExist (Variables|Default|GetSaveGameSlotName)))
  (if _returnvalue
    (bind _returnvalue_2 (SaveGame|LoadGamefromSlot (Variables|Default|GetSaveGameSlotName)))
    (bind _asworld_save_game (Utilities|Casting|CastToWorldSaveGame _returnvalue_2))
    (Variables|Default|SetSaveGame _asworld_save_game)
    (CallFunction|LoadWorldData)
    (CallFunction|LoadPlayerData)
    (Development|PrintString "Game Loaded." true false "(R=0.116623,G=1.000000,B=0.000000,A=1.000000)")))

(event Custom|DeleteSaveGame
  (bind _returnvalue (SaveGame|DoesSaveGameExist (Variables|Default|GetSaveGameSlotName)))
  (if _returnvalue
    (bind _returnvalue_2 (SaveGame|DeleteGameinSlot (Variables|Default|GetSaveGameSlotName)))
    (if _returnvalue_2
      (Development|PrintString "Save Game Deleted." true false "(R=1.000000,G=0.000000,B=0.000000,A=1.000000)"))))

(fn LoadPlayerData
  (Class|BpiPlayer|SetPlayerData(Message) (Game|Player|GetPlayerPawn 0) (Variables|/Game/Game/Blueprints/SaveGame/WorldSaveGame.WorldSaveGame_C|GetPlayerSave (Variables|Default|GetSaveGame))))

(fn LoadWorldData
  (Utilities|FlowControl|Sequence
    (:then_0
      (bind _outactors (Actor|GetAllActorsOfClass "/Game/Game/Blueprints/Items/ItemBase.ItemBase_C"))
      (for _array_element _outactors
        (Actor|DestroyActor _array_element))
      (for _array_element_2 (Variables|/Game/Game/Blueprints/SaveGame/WorldSaveGame.WorldSaveGame_C|GetWorldItemsSave (Variables|Default|GetSaveGame))
        (bind _returnvalue (Game|SpawnActorfromClass (.ItemClass (Utilities|Struct|BreakItemStruct _array_element_2)) (Utilities|Struct|BreakItemDataStruct (.ItemData (Utilities|Struct|BreakItemStruct _array_element_2))) "Undefined" 0 0))
        (Class|BpiItem|OnLoadGame(Message) _returnvalue _array_element_2)))
    (:then_1
      (bind _outactors_2 (Actor|GetAllActorsOfClass "/Game/Game/Blueprints/Interactable/Interactable.Interactable_C"))
      (for _array_element_3 _outactors_2
        (bind _data (Class|BpiInteractable|GetInteractableData(Message) _array_element_3))
        (bind _array_element_4 (Utilities|Array|ForEachLoopwithBreak (Variables|/Game/Game/Blueprints/SaveGame/WorldSaveGame.WorldSaveGame_C|GetWorldInteractableSave (Variables|Default|GetSaveGame)) :!label _label)
          (:LoopBody
            (if (Utilities|Enum|Equal(Enum) (Utilities|Struct|BreakObjectDataStruct _array_element_4) (Utilities|Struct|BreakObjectDataStruct _data))
              (Class|BpiInteractable|SetInteractableData(Message) _array_element_3 _array_element_4)
              (goto _label Break))))))))

(fn CollectWorldData
  (bind _savegame (Variables|Default|GetSaveGame))
  (Utilities|Array|Clear (Variables|/Game/Game/Blueprints/SaveGame/WorldSaveGame.WorldSaveGame_C|GetWorldItemsSave _savegame))
  (Utilities|Array|Clear (Variables|/Game/Game/Blueprints/SaveGame/WorldSaveGame.WorldSaveGame_C|GetWorldInteractableSave _savegame))
  (Utilities|FlowControl|Sequence
    (:then_0
      (bind _outactors (Actor|GetAllActorsOfClass "/Game/Game/Blueprints/Items/ItemBase.ItemBase_C"))
      (for _array_element _outactors
        (bind _item (Class|BpiItem|GetItemData(Message) _array_element))
        (Utilities|Array|Add (Variables|/Game/Game/Blueprints/SaveGame/WorldSaveGame.WorldSaveGame_C|GetWorldItemsSave (Variables|Default|GetSaveGame)) _item)))
    (:then_1
      (bind _outactors_2 (Actor|GetAllActorsOfClass "/Game/Game/Blueprints/Interactable/Interactable.Interactable_C"))
      (for _array_element_2 _outactors_2
        (bind _data (Class|BpiInteractable|GetInteractableData(Message) _array_element_2))
        (Utilities|Array|Add (Variables|/Game/Game/Blueprints/SaveGame/WorldSaveGame.WorldSaveGame_C|GetWorldInteractableSave (Variables|Default|GetSaveGame)) _data)))))

(fn CollectPlayerData
  (bind _playersavedata (Class|BpiPlayer|GetPlayerData(Message) (Game|Player|GetPlayerPawn 0)))
  (Variables|/Game/Game/Blueprints/SaveGame/WorldSaveGame.WorldSaveGame_C|SetPlayerSave (Variables|Default|GetSaveGame) _playersavedata))

(fn GetMouseSens
  (return (.MouseSens (Utilities|Struct|BreakGameSettingsStruct (Variables|Default|GetGameSettings)))))