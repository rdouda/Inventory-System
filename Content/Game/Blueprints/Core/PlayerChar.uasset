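; Player character that handles movement, toggled run and crouch with a timeline camera height blend, and mouse look scaled by game sensitivity.
; A line trace picks up items into the hand or inventory, or triggers interactables.
; InventorySystem and HandleComponent handle hotkey equipping, stashing, dropping and using held items.
; Save functions pack and restore transform, inventory, crouch state and held item; packing destroys the held actor.
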(event EventBeginPlay
  (bind _game (CallFunction|GetGame))
  (Variables|Default|SetGame _game))

(event EventGrabItem
  (params (Index :type Integer))
  ;[0.1976 0.6047 1] Inventory
  (bind (_return_value _object) (Default|GetGrabbedObject (Variables|Default|GetHandleComponent)))
  (if _return_value
    (bind (_return_value_2 _output) (Default|GetItem (Variables|Default|GetInventorySystem) Index))
    (if _return_value_2
      (bind _return_value_3 (Default|AddItem (Variables|Default|GetInventorySystem) _object))
      (if _return_value_3
        (Default|SetObjectandTarget (Variables|Default|GetHandleComponent) (Variables|Default|GetGrabLocation) _output)))
    (else
      (bind (_return_value_4 _output_2) (Default|GetItem (Variables|Default|GetInventorySystem) Index))
      (if _return_value_4
        (Default|SetObjectandTarget (Variables|Default|GetHandleComponent) (Variables|Default|GetGrabLocation) _output_2)))))

(event EventTick
  (params (DeltaSeconds :type Float%20%28single-precision%29)))

(event EventAddItem
  (params (Item :type Item%20Base%20Object%20Reference))
  ;[0.1976 0.6047 1] Inventory
  (Default|AddItem (Variables|Default|GetInventorySystem) Item))

(event EventSetPlayerData
  (params (PlayerSaveData :type Player%20Save%20Struct%20Structure))
  (bind (_transform _inventory _holdingitem _iscrouched) (Utilities|Struct|BreakPlayerSaveStruct PlayerSaveData))
  (Utilities|FlowControl|Sequence
    (:then_0
      (if _iscrouched
        (Character|Crouch)
        (Transformation|SetRelativeLocation (Variables|Default|GetSpringArm) (Variables|Camera|GetCrouchCameraHeight) false false)))
    (:then_1
      (Transformation|SetActorTransform (Math|Transform|MakeTransform (.location _transform) "0, 0, 0" (.scale _transform)))
      (Pawn|SetControlRotation (Pawn|GetController) (.rotation _transform))
      (CallFunction|SetInventory _inventory)
      (Utilities|IsValidClass (.ItemClass (Utilities|Struct|BreakItemStruct _holdingitem))
        (:Is%20Valid
          (Default|SetObjectandTarget (Variables|Default|GetHandleComponent) (Variables|Default|GetGrabLocation) _holdingitem))))))

(event EventSetInventory
  (params (New%20Inventory :type Array%20of%20Item%20Struct%20Structures))
  ;[0.1976 0.6047 1] Inventory
  (Variables|/Game/Game/Blueprints/InventorySystem/InventorySystemComponent.InventorySystemComponent_C|SetInventory (Variables|Default|GetInventorySystem) New%20Inventory))

(event Input|ActionEvents|InputActionDrop
  (params (Key :type Key%20Structure :default "None"))
  ;[0.4562 1 0.8172] Object Interaction
  (:Pressed
    (Default|ReleaseObject (Variables|Default|GetHandleComponent))))

(event Input|ActionEvents|InputActionCrouch
  (params (Key :type Key%20Structure :default "None"))
  ;[0.3991 0.6626 1] Movements
  (:Pressed
    (if (Variables|Default|GetbIsCrouched)
      (Character|UnCrouch)
      (bind _value (Timeline|Timeline_0 Reverse)
        (:Update
          (Transformation|SetRelativeLocation (Variables|Default|GetSpringArm) (Math|Vector|Lerp(Vector) (Variables|Default|GetUnCrouchCameraHeight) (Variables|Camera|GetCrouchCameraHeight) _value) false false)))
      (else
        (Character|Crouch)
        (Utilities|FlowControl|Sequence
          (:then_0
            (Variables|/Script/Engine.CharacterMovementComponent|SetMaxWalkSpeed (Variables|Character|GetCharacterMovement) 2.3e+02)
            (Variables|Character|SetRunning false))
          (:then_1
            (Timeline|Timeline_0 Play)))))))

(event Input|ActionEvents|InputActionRun
  (params (Key :type Key%20Structure :default "None"))
  ;[0.3991 0.6626 1] Movements
  (:Pressed
    (if (Variables|Default|GetbIsCrouched)
      (Utilities|FlowControl|Sequence
        (:then_0
          (Character|UnCrouch)
          (bind _value (Timeline|Timeline_0 Reverse)
            (:Update
              (Transformation|SetRelativeLocation (Variables|Default|GetSpringArm) (Math|Vector|Lerp(Vector) (Variables|Default|GetUnCrouchCameraHeight) (Variables|Camera|GetCrouchCameraHeight) _value) false false))))
        (:then_1
          (Variables|/Script/Engine.CharacterMovementComponent|SetMaxWalkSpeed (Variables|Character|GetCharacterMovement) 4.2e+02)
          (Variables|Character|SetRunning true)))
      (elif (Variables|Character|GetRunning)
        (Variables|/Script/Engine.CharacterMovementComponent|SetMaxWalkSpeed (Variables|Character|GetCharacterMovement) 2.3e+02)
        (Variables|Character|SetRunning false)
        (else
          (Variables|/Script/Engine.CharacterMovementComponent|SetMaxWalkSpeed (Variables|Character|GetCharacterMovement) 4.2e+02)
          (Variables|Character|SetRunning true))))))

(event Input|ActionEvents|InputActionJump
  (params (Key :type Key%20Structure :default "None"))
  ;[0.3991 0.6626 1] Movements
  (:Pressed
    (Character|Jump))
  (:Released
    (Character|StopJumping)))

(event Input|ActionEvents|InputActionInteract
  (params (Key :type Key%20Structure :default "None"))
  ;[0.4562 1 0.8172] Object Interaction
  (:Pressed
    (bind (_return_value _hitactor) (CallFunction|LineTrace 3e+02 "ForDuration"))
    (if _return_value
      (Utilities|FlowControl|Sequence
        (:then_0
          (if (Utilities|DoesObjectImplementInterface _hitactor "/Game/Game/Blueprints/Items/bpi_item.bpi_item_C")
            (bind _asitem_base (Utilities|Casting|CastToItemBase _hitactor))
            (bind _return_value_2 (Default|GetGrabbedObject (Variables|Default|GetHandleComponent)))
            (if _return_value_2
              (Default|AddItem (Variables|Default|GetInventorySystem) _asitem_base)
              (else
                (bind _item (Class|BpiItem|GetItemData(Message) _asitem_base))
                (Default|SetObjectandTarget (Variables|Default|GetHandleComponent) (Variables|Default|GetGrabLocation) _item)
                (Actor|DestroyActor _asitem_base)))))
        (:then_1
          (if (Utilities|DoesObjectImplementInterface _hitactor "/Game/Game/Blueprints/Interactable/bpi_interactable.bpi_interactable_C")
            (Class|BpiInteractable|Interact(Message) _hitactor)))))))

(event Input|ActionEvents|InputActionStash
  (params (Key :type Key%20Structure :default "None"))
  ;[0.4562 1 0.8172] Object Interaction
  (:Pressed
    (bind (_return_value _object) (Default|GetGrabbedObject (Variables|Default|GetHandleComponent)))
    (if _return_value
      (Default|AddItem (Variables|Default|GetInventorySystem) _object))))

(event Input|ActionEvents|InputActionLMB
  (params (Key :type Key%20Structure :default "None"))
  ;[0.4562 1 0.8172] Object Interaction
  (:Pressed
    (bind (_return_value _object) (Default|GetGrabbedObject (Variables|Default|GetHandleComponent)))
    (if _return_value
      (Class|BpiItem|OnInteract(Message) _object))))

(event Input|AxisEvents|InputAxisMoveForward
  (params (AxisValue :type Float%20%28single-precision%29))
  ;[0.3991 0.6626 1] Movements
  (Pawn|Input|AddMovementInput (CallFunction|ForwardVector) AxisValue false))

(event Input|AxisEvents|InputAxisMoveRight
  (params (AxisValue :type Float%20%28single-precision%29))
  ;[0.3991 0.6626 1] Movements
  (Pawn|Input|AddMovementInput (CallFunction|RightVector) AxisValue false))

(event Input|AxisEvents|InputAxisTurn
  (params (AxisValue :type Float%20%28single-precision%29))
  ;[0.3991 0.6626 1] Movements
  (Pawn|Input|AddControllerYawInput (CallFunction|TurnValue)))

(event Input|AxisEvents|InputAxisLookUp
  (params (AxisValue :type Float%20%28single-precision%29))
  ;[0.3991 0.6626 1] Movements
  (Pawn|Input|AddControllerPitchInput (CallFunction|LookUpValue)))

(event Input|KeyboardEvents|4
  (params (Key :type Key%20Structure :default "None"))
  ;[0.4562 1 0.8172] Object Interaction
  (:Pressed
    (CallFunction|GrabItem 3)))

(event Input|KeyboardEvents|1
  (params (Key :type Key%20Structure :default "None"))
  ;[0.4562 1 0.8172] Object Interaction
  (:Pressed
    (CallFunction|GrabItem)))

(event Input|KeyboardEvents|2
  (params (Key :type Key%20Structure :default "None"))
  ;[0.4562 1 0.8172] Object Interaction
  (:Pressed
    (CallFunction|GrabItem 1)))

(event Input|KeyboardEvents|3
  (params (Key :type Key%20Structure :default "None"))
  ;[0.4562 1 0.8172] Object Interaction
  (:Pressed
    (CallFunction|GrabItem 2)))

(event Input|KeyboardEvents|5
  (params (Key :type Key%20Structure :default "None"))
  ;[0.4562 1 0.8172] Object Interaction
  (:Pressed
    (CallFunction|GrabItem 4)))

(event Input|KeyboardEvents|6
  (params (Key :type Key%20Structure :default "None"))
  ;[0.4562 1 0.8172] Object Interaction
  (:Pressed
    (CallFunction|GrabItem 5)))

(fn ConstructionScript)

(fn LookUpValue
  (return (* (Input|AxisValues|GetLookUp) (Default|GetMouseSens (Variables|Default|GetGame)))))

(fn TurnValue
  (return (* (Input|AxisValues|GetTurn) (Default|GetMouseSens (Variables|Default|GetGame)))))

(fn ForwardVector
  (return (Math|Vector|GetForwardVector (Math|Rotator|MakeRotator 0.0 0.0 (.yaw (Pawn|GetControlRotation :!class /Script/Engine.Pawn))))))

(fn RightVector
  (return (Math|Vector|GetRightVector (Math|Rotator|MakeRotator 0.0 0.0 (.yaw (Pawn|GetControlRotation :!class /Script/Engine.Pawn))))))

(fn GetPlayerData
  (bind _returnvalue (Transformation|GetActorTransform))
  (Utilities|FlowControl|Sequence
    (:then_0
      (bind (_return_value _object) (Default|GetGrabbedObject (Variables|Default|GetHandleComponent)))
      (if _return_value
        (bind _item (Class|BpiItem|GetItemData(Message) _object))
        (LocalVariables|SetItemData _item)
        (bind _returnvalue_2 (Default|ReleaseObject (Variables|Default|GetHandleComponent)))
        (Actor|DestroyActor _returnvalue_2)))
    (:then_1
      (return (Utilities|Struct|MakePlayerSaveStruct (Math|Transform|MakeTransform (.location _returnvalue) (Pawn|GetControlRotation :!class /Script/Engine.Pawn) (.scale _returnvalue)) (Variables|/Game/Game/Blueprints/InventorySystem/InventorySystemComponent.InventorySystemComponent_C|GetInventory (Variables|Default|GetInventorySystem)) (LocalVariables|GetItemData) (Variables|Default|GetbIsCrouched))))))