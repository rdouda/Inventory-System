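; Actor component that gives its owner a fixed-size, slot-based inventory with item stacking, sized on BeginPlay.
; AddItem puts an item's struct into a matching non-full stack or else the first empty slot (name "None"), destroying the item actor on success.
; GetItem decrements the stack at an index, clears it at zero and returns the item struct.
; Every tick prints all slots on screen as a debug view.
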(event EventBeginPlay
  (Utilities|InitializeInventorySystem))

(event EventTick
  (params (DeltaSeconds :type Float%20%28single-precision%29))
  (Utilities|ShowInventory))

(fn AddItem
  (params (Item :type Item%20Base%20Object%20Reference))
  (bind _item (Class|BpiItem|GetItemData(Message) Item))
  (Utilities|FindAppropriateSlotforItem _item
    (:Item%20Added
      (Actor|DestroyActor Item)
      (return true))
    (:Inventory%20Full
      (return false))))

(fn GetItem
  (params (Index :type Integer))
  (bind _output (Utilities|GetItemfromSlot Index)
    (:ItemFound
      (return true _output))
    (:ItemNotFound
      (return false ""))))