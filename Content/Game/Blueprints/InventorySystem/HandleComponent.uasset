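; Actor component in the inventory system that holds a spawned item in place at a target scene component, like a handheld object.
; SetObjectAndTarget spawns the item from its item struct, copies in the data and disables mesh physics.
; Tick interpolates the item mesh's transform toward the target every frame.
; ReleaseObject replaces the held item with a fresh spawn at the target carrying the same data, destroys the original and returns the new actor.
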(event EventBeginPlay)

(event EventTick
  (params (DeltaSeconds :type Float%20%28single-precision%29))
  (CallFunction|GrabObjectatTransform DeltaSeconds 22.0))

(fn GrabObjectatTransform
  (params (DeltaTime :type Float%20%28single-precision%29) (InterpSpeed :type Float%20%28single-precision%29))
  (bind _object (Variables|Default|GetObject))
  (bind _itemmesh (Variables|/Game/Game/Blueprints/Items/ItemBase.ItemBase_C|GetItemMesh _object))
  (if (and (Utilities|IsValid (Variables|Default|GetObject)) (Utilities|IsValid (Variables|Default|GetTarget)))
    (Transformation|SetWorldTransform _itemmesh (Class|KismetMathLibrary|TInterpto (Transformation|GetWorldTransform _itemmesh) (Transformation|GetWorldTransform (Variables|Default|GetTarget)) DeltaTime InterpSpeed) false false)))

(fn SetObjectandTarget
  (params (Target :type Scene%20Component%20Object%20Reference) (ItemStruct :type Item%20Struct%20Structure%20%28by%20ref%29))
  (bind _returnvalue (Components|GetOwner))
  (bind _returnvalue_2 (Game|SpawnActorfromClass (Utilities|Struct|BreakItemStruct ItemStruct) (Transformation|GetActorTransform _returnvalue) "Undefined" _returnvalue 0))
  (bind _output_get (Variables|Default|SetObject _returnvalue_2))
  (Class|BpiItem|SetItemData(Message) _output_get ItemStruct)
  (Physics|SetSimulatePhysics (Variables|/Game/Game/Blueprints/Items/ItemBase.ItemBase_C|GetItemMesh _output_get) false)
  (Variables|Default|SetTarget Target))

(fn ReleaseObject
  (Utilities|IsValid (Variables|Default|GetObject)
    (:Is%20Valid
      (bind _item (Class|BpiItem|GetItemData(Message) (Variables|Default|GetObject)))
      (bind _returnvalue (Game|SpawnActorfromClass (Utilities|Struct|BreakItemStruct _item) (Transformation|GetWorldTransform (Variables|Default|GetTarget)) "Undefined" 0 0))
      (Class|BpiItem|SetItemData(Message) _returnvalue _item)
      (Variables|Default|SetTarget 0)
      (Actor|DestroyActor (Variables|Default|GetObject))
      (return _returnvalue))))

(fn GetGrabbedObject
  (bind _object (Variables|Default|GetObject))
  (return (Utilities|IsValid _object) _object))