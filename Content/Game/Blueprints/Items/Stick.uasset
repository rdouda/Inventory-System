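; Stick is an item Blueprint that supplies its item data and restores its world placement when a game loads.
; GetItemData rebuilds the item struct from the stored fields, substituting the mesh's current world transform.
; OnLoadGame applies the saved transform back to the mesh, while SetItemData is left empty.
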(event EventBeginPlay)

(event Collision|EventActorBeginOverlap
  (params (OtherActor :type Actor%20Object%20Reference)))

(event EventTick
  (params (DeltaSeconds :type Float%20%28single-precision%29)))

(event EventOnLoadGame
  (params (Data :type Item%20Struct%20Structure))
  (Transformation|SetWorldTransform (Variables|Default|GetItemMesh) (.Transform (Utilities|Struct|BreakItemDataStruct (Utilities|Struct|BreakItemStruct Data))) false false))

(event EventSetItemData
  (params (ItemData :type Item%20Struct%20Structure)))

(fn ConstructionScript
  (|CallParentFunction))

(fn GetItemData
  (bind _itemstruct (Variables|Default|GetItemStruct))
  (bind (_itemclass _itemname _maxstacksize _stackcount _isstackable _itemtexture2d _itemdata) (Utilities|Struct|BreakItemStruct _itemstruct))
  (return (Utilities|Struct|MakeItemStruct _itemclass _itemname _maxstacksize _stackcount _isstackable _itemtexture2d (Utilities|Struct|MakeItemDataStruct (Transformation|GetWorldTransform (Variables|Default|GetItemMesh)) (.boolslot_1 _itemdata) (.boolslot_2 _itemdata) (.intslot_1 _itemdata) (.intslot_2 _itemdata) (.floatslot_1 _itemdata) (.floatslot_2 _itemdata)))))